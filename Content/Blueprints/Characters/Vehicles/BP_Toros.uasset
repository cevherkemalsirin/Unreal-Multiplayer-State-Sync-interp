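; BP_Toros is a vehicle Blueprint that animates the height of its four wheel components to follow the suspension.
; Each Tick runs the parent logic, then sets each wheel's relative Z to its negated SuspensionLengths entry, keeping X and Y and sweeping the move.
; Array indices map to wheels in diagonal pairs: LF, RB, RF, LB.
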(event EventBeginPlay)

(event Collision|EventActorBeginOverlap
  (params (OtherActor :type Actor%20Object%20Reference)))

(event EventTick
  (params (DeltaSeconds :type Float%20%28single-precision%29))
  (|CallParentFunction DeltaSeconds)
  (bind _index (Utilities|FlowControl|ForLoopwithBreak 0 3)
    (:LoopBody
      (Transformation|SetRelativeLocation (Utilities|Select :Index _index :Option%200 (Variables|Default|Getwheel_LF) :Option%201 (Variables|Default|Getwheel_RB) :Option%202 (Variables|Default|Getwheel_RF) :Option%203 (Variables|Default|Getwheel_LB)) (Math|Vector|MakeVector (.x (Variables|/Script/Engine.SceneComponent|GetRelativeLocation (Utilities|Select :Index _index :Option%200 (Variables|Default|Getwheel_LF) :Option%201 (Variables|Default|Getwheel_RB) :Option%202 (Variables|Default|Getwheel_RF) :Option%203 (Variables|Default|Getwheel_LB)))) (.y (Variables|/Script/Engine.SceneComponent|GetRelativeLocation (Utilities|Select :Index _index :Option%200 (Variables|Default|Getwheel_LF) :Option%201 (Variables|Default|Getwheel_RB) :Option%202 (Variables|Default|Getwheel_RF) :Option%203 (Variables|Default|Getwheel_LB)))) (* (Utilities|Array|Get(acopy) (Variables|Default|GetsuspensionLengths) _index) -1.0)) true false))))

(fn ConstructionScript)